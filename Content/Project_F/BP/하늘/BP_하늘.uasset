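; Space sky actor (하늘) that draws a configurable gas-cloud and starfield backdrop on a sphere.
; The construction script creates a dynamic material for SpaceSphere, then UpdateMaterials pushes the gradient, gas and starfield settings into it and calls SpaceSphereUpdated.
; An optional sun branch rotates SunRoot and sets sun and flare parameters, but those materials' creation nodes are disconnected.
; The asteroid branch is empty, and no gameplay events run.
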(event EventBeginPlay)

(event Collision|EventActorBeginOverlap
  (params (OtherActor :type Actor%20Object%20Reference)))

(event EventTick
  (params (DeltaSeconds :type Float%20%28single-precision%29)))

(fn ConstructionScript
  (bind _spacesphere (Variables|Default|GetSpaceSphere))
  (Utilities|FlowControl|Sequence
    (:then_0
      (bind _returnvalue (Rendering|Material|CreateDynamicMaterialInstance _spacesphere 0 (Rendering|Material|GetMaterial _spacesphere 0) "None" :!class /Script/Engine.PrimitiveComponent))
      (Variables|Default|SetSpaceSphereMaterial _returnvalue))
    (:then_3
      (CallFunction|UpdateMaterials))))

(fn UpdateMaterials
  (bind _spacespherematerial (Variables|Default|GetSpaceSphereMaterial))
  (bind _solarflarematerial (Variables|Default|GetSolarFlareMaterial))
  (bind _sun_rotation (Variables|Sun|GetSun%20rotation))
  (bind _sunmaterial (Variables|Default|GetSunMaterial))
  (bind _spacespherematerial_2 (Variables|Default|GetSpaceSphereMaterial))
  (bind (_x _y) (Math|Vector2D|BreakVector2D _sun_rotation))
  (Utilities|FlowControl|Sequence
    (:then_0
      (if (Variables|GasClouds|GetHas%20Asteroids)
        _))
    (:then_1
      (if (Variables|Sun|GetHas%20sun)
        (Utilities|FlowControl|Sequence
          (:then_0
            (Transformation|SetRelativeRotation (Variables|Default|GetSunRoot) (Math|Rotator|MakeRotator 0.0 _y _x) false false))
          (:then_5
            (Utilities|FlowControl|Sequence
              (:then_0
                (Rendering|Material|SetVectorParameterValue _sunmaterial "Inner colour" (Variables|Sun|GetInner%20colour) :!class /Script/Engine.MaterialInstanceDynamic))
              (:then_1
                (Rendering|Material|SetVectorParameterValue _sunmaterial "Outer colour" (Variables|Sun|GetOuter%20colour) :!class /Script/Engine.MaterialInstanceDynamic))
              (:then_2
                (Rendering|Material|SetScalarParameterValue _sunmaterial "Brightness" (Variables|Sun|GetBrightness) :!class /Script/Engine.MaterialInstanceDynamic))
              (:then_3
                (Rendering|Material|SetScalarParameterValue _sunmaterial "Fresnel power" (Variables|Sun|GetColour%20balance) :!class /Script/Engine.MaterialInstanceDynamic))
              (:then_4
                (Rendering|Material|SetScalarParameterValue _sunmaterial "Sunspot strength" (Variables|Sun|GetSunspot%20strength) :!class /Script/Engine.MaterialInstanceDynamic))))
          (:then_6
            (if (Variables|Sun|GetSolar%20flares)
              (Utilities|FlowControl|Sequence
                (:then_0
                  (Rendering|Material|SetVectorParameterValue _solarflarematerial "Colour 1" (Variables|Sun|GetInner%20colour) :!class /Script/Engine.MaterialInstanceDynamic))
                (:then_1
                  (Rendering|Material|SetVectorParameterValue _solarflarematerial "Colour 2" (Variables|Sun|GetOuter%20colour) :!class /Script/Engine.MaterialInstanceDynamic))
                (:then_3
                  (Rendering|Material|SetScalarParameterValue _solarflarematerial "Brightness" (Variables|Sun|GetBrightness) :!class /Script/Engine.MaterialInstanceDynamic))
                (:then_4
                  (Rendering|Material|SetScalarParameterValue _solarflarematerial "Opacity" (Variables|Sun|GetSolar%20flare%20opacity) :!class /Script/Engine.MaterialInstanceDynamic)))
              (else
                (CallFunction|SafeDestroyActorComponent)))))))
    (:then_2
      (Utilities|FlowControl|Sequence
        (:then_0
          (Rendering|Material|SetVectorParameterValue _spacespherematerial_2 "1. Top" (Variables|Gasclouds|GetTop) :!class /Script/Engine.MaterialInstanceDynamic))
        (:then_1
          (Rendering|Material|SetVectorParameterValue _spacespherematerial_2 "2. Middle" (Variables|Gasclouds|GetMiddle) :!class /Script/Engine.MaterialInstanceDynamic))
        (:then_2
          (Rendering|Material|SetVectorParameterValue _spacespherematerial_2 "3. Bottom" (Variables|Gasclouds|GetBottom) :!class /Script/Engine.MaterialInstanceDynamic))
        (:then_3
          (Rendering|Material|SetScalarParameterValue _spacespherematerial_2 "Dust falloff" (Variables|Gasclouds|GetGas%20cloud%20falloff) :!class /Script/Engine.MaterialInstanceDynamic))
        (:then_4
          (Rendering|Material|SetScalarParameterValue _spacespherematerial_2 "Dust noise power" (Variables|Gasclouds|GetGas%20turbulence%20falloff) :!class /Script/Engine.MaterialInstanceDynamic))
        (:then_5
          (Rendering|Material|SetScalarParameterValue _spacespherematerial_2 "Dust noise tiling" (Variables|Gasclouds|GetGas%20turbulence%20scale) :!class /Script/Engine.MaterialInstanceDynamic))
        (:then_6
          (Rendering|Material|SetScalarParameterValue _spacespherematerial_2 "Add heat" (Variables|Gasclouds|GetGas%20heat) :!class /Script/Engine.MaterialInstanceDynamic))
        (:then_7
          (Rendering|Material|SetScalarParameterValue _spacespherematerial_2 "Hue spin X" (Variables|Gasclouds|GetHue%20spin%20X) :!class /Script/Engine.MaterialInstanceDynamic))
        (:then_8
          (Rendering|Material|SetScalarParameterValue _spacespherematerial_2 "Hue spin Y" (Variables|Gasclouds|GetHue%20spin%20Y) :!class /Script/Engine.MaterialInstanceDynamic))
        (:then_9
          (Rendering|Material|SetTextureParameterValue _spacespherematerial_2 "Gas texture" (Variables|Gasclouds|GetGas%20texture)))))
    (:then_3
      (Utilities|FlowControl|Sequence
        (:then_0
          (Rendering|Material|SetScalarParameterValue _spacespherematerial "Starfield falloff" (Variables|Starfield|GetStarfield%20falloff) :!class /Script/Engine.MaterialInstanceDynamic))
        (:then_1
          (Rendering|Material|SetScalarParameterValue _spacespherematerial "Starfield tiling" (Variables|Starfield|GetStarfield%20density) :!class /Script/Engine.MaterialInstanceDynamic))))
    (:then_4
      (Default|CallSpaceSphereUpdated))))

(fn SafeDestroyActorComponent
  (params (ActorComponent :type Actor%20Component%20Object%20Reference))
  (if (!= ActorComponent 0)
    (Components|DestroyComponent ActorComponent)))