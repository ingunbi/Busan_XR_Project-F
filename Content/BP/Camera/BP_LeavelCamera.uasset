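; BP_LeavelCamera is a shared side-view level camera that keeps two players framed in a single shot.
; After a short startup delay it caches Player01 and Player02 from BP_ThirdPersonGameMode.
; Each tick it moves to the players' midpoint in X and Z within fixed bounds, keeping Y constant.
; It also widens the camera's field of view with their horizontal separation, clamped to a set range.
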(event EventBeginPlay
  (Utilities|FlowControl|Delay 3.0)
  (bind _asbp_third_person_game_mode (Utilities|Casting|CastToBP_ThirdPersonGameMode (Game|GetGameMode)))
  (Utilities|IsValid (Variables|/Game/ThirdPerson/Blueprints/BP_ThirdPersonGameMode.BP_ThirdPersonGameMode_C|GetPlayer_01 _asbp_third_person_game_mode)
    (:Is%20Valid
      (Variables|Default|SetP1 (Variables|/Game/ThirdPerson/Blueprints/BP_ThirdPersonGameMode.BP_ThirdPersonGameMode_C|GetPlayer_01 _asbp_third_person_game_mode))
      (Utilities|IsValid (Variables|/Game/ThirdPerson/Blueprints/BP_ThirdPersonGameMode.BP_ThirdPersonGameMode_C|GetPlayer_02 _asbp_third_person_game_mode)
        (:Is%20Valid
          (Variables|Default|SetP2 (Variables|/Game/ThirdPerson/Blueprints/BP_ThirdPersonGameMode.BP_ThirdPersonGameMode_C|GetPlayer_02 _asbp_third_person_game_mode)))))))

(event EventTick
  (params (DeltaSeconds :type Float%20%28single-precision%29))
  (bind _p2 (Variables|Default|GetP2))
  (bind _p1 (Variables|Default|GetP1))
  (bind _returnvalue (Transformation|GetActorLocation _p2))
  (bind _returnvalue_2 (Transformation|GetActorLocation _p1))
  (bind (_x _y _z) (Math|Vector|BreakVector _returnvalue))
  (bind (_x_2 _y_2 _z_2) (Math|Vector|BreakVector _returnvalue_2))
  (if (and (Utilities|IsValid _p1) (Utilities|IsValid _p2))
    (Transformation|SetActorLocation (Math|Vector|MakeVector (Math|Float|Clamp(Float) (/ (+ _x _x_2) 2.0) 0.0 3e+03) (.Y (Math|Vector|BreakVector (Transformation|GetActorLocation))) (Math|Float|Clamp(Float) (/ (+ _z _z_2) 2.0) 0.0 1e+03)) false false)
    (Camera|SetFieldOfView (Variables|CameraActor|GetCameraComponent) (Math|Float|Clamp(Float) (Math|Float|Absolute(Float) (* (- (.x (Transformation|GetActorLocation (Variables|Default|GetP1))) (.x (Transformation|GetActorLocation (Variables|Default|GetP2)))) 0.03)) 9e+01 125.0))))

(fn ConstructionScript)