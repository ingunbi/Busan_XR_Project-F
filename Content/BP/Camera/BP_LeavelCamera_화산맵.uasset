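; Shared two-player level camera for the volcano map that frames both characters by following their midpoint.
; Shortly after BeginPlay, it caches Player01 and Player02 from BP_ThirdPersonGameMode.
; Each Tick it moves to their clamped average X and Z with a height offset, keeping Y unchanged.
; It also widens the field of view as their horizontal X separation grows, within a clamped range.
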(event EventBeginPlay
  (Utilities|FlowControl|Delay 0.3)
  (bind _asbp_third_person_game_mode (Utilities|Casting|CastToBP_ThirdPersonGameMode (Game|GetGameMode)))
  (Utilities|IsValid (Variables|/Game/ThirdPerson/Blueprints/BP_ThirdPersonGameMode.BP_ThirdPersonGameMode_C|GetPlayer_01 _asbp_third_person_game_mode)
    (:Is%20Valid
      (Variables|Default|SetP1 (Variables|/Game/ThirdPerson/Blueprints/BP_ThirdPersonGameMode.BP_ThirdPersonGameMode_C|GetPlayer_01 _asbp_third_person_game_mode))
      (Utilities|IsValid (Variables|/Game/ThirdPerson/Blueprints/BP_ThirdPersonGameMode.BP_ThirdPersonGameMode_C|GetPlayer_02 _asbp_third_person_game_mode)
        (:Is%20Valid
          (Variables|Default|SetP2 (Variables|/Game/ThirdPerson/Blueprints/BP_ThirdPersonGameMode.BP_ThirdPersonGameMode_C|GetPlayer_02 _asbp_third_person_game_mode)))))))

(event EventTick
  (params (DeltaSeconds :type Float%20%28single-precision%29))
  (bind _returnvalue (Transformation|GetActorLocation))
  (bind _p2 (Variables|Default|GetP2))
  (bind _p1 (Variables|Default|GetP1))
  (bind _returnvalue_2 (Transformation|GetActorLocation _p2))
  (bind _returnvalue_3 (Transformation|GetActorLocation _p1))
  (bind _y (Math|Vector|BreakVector _returnvalue))
  (bind (_x _y_2 _z) (Math|Vector|BreakVector _returnvalue_2))
  (bind (_x_2 _y_3 _z_2) (Math|Vector|BreakVector _returnvalue_3))
  (bind _returnvalue_4 (+ _z _z_2))
  (bind _returnvalue_5 (+ _x _x_2))
  (bind _returnvalue_6 (/ _returnvalue_4 2.0))
  (bind _returnvalue_7 (/ _returnvalue_5 2.0))
  (bind _returnvalue_8 (Math|Float|Clamp(Float) _returnvalue_7 -2e+03 3e+03))
  (bind _returnvalue_9 (Math|Float|Clamp(Float) _returnvalue_6 -5e+03 1e+03))
  (bind _returnvalue_10 (Math|Vector|MakeVector _returnvalue_8 _y _returnvalue_9))
  (if (and (Utilities|IsValid _p1) (Utilities|IsValid _p2))
    (Transformation|SetActorLocation (Math|Vector|MakeVector (.x _returnvalue_10) (.y _returnvalue_10) (+ (.z _returnvalue_10) 5e+02)) false false)
    (Camera|SetFieldOfView (Variables|CameraActor|GetCameraComponent) (Math|Float|Clamp(Float) (Math|Float|Absolute(Float) (* (- (.x (Transformation|GetActorLocation (Variables|Default|GetP1))) (.x (Transformation|GetActorLocation (Variables|Default|GetP2)))) 0.03)) 9e+01 1.2e+02))))

(fn ConstructionScript)